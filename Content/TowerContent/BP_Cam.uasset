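; BP_Cam is a player-controlled camera that also holds an Energy resource, apparently for a tower game.
; Axis inputs move it along local X and Y scaled by MoveCamSpeed, and ZoomCam changes the spring arm length in fixed steps without clamping.
; CalculateEnergy deducts a cost only when enough Energy remains and returns whether it succeeded.
; Tick prints the current Energy to screen every frame.
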(event EventBeginPlay)

(event EventTick
  (params (DeltaSeconds :type Float%20%28single-precision%29))
  (Development|PrintString (Utilities|String|ToString(Float) (Variables|Default|GetEnergy))))

(event Input|AxisEvents|InputAxisMoveForward
  (params (AxisValue :type Float%20%28single-precision%29))
  (Transformation|AddActorLocalOffset (Math|Vector|MakeVector (* AxisValue (Variables|Default|GetMoveCamSpeed)) 0.0 0.0) false false))

(event Input|AxisEvents|InputAxisMoveRight
  (params (AxisValue :type Float%20%28single-precision%29))
  (Transformation|AddActorLocalOffset (Math|Vector|MakeVector 0.0 (* AxisValue (Variables|Default|GetMoveCamSpeed)) 0.0) false false))

(event Input|AxisEvents|InputAxisZoomCam
  (params (AxisValue :type Float%20%28single-precision%29))
  (if (!= AxisValue 0.0)
    (Variables|/Script/Engine.SpringArmComponent|SetTargetArmLength (Variables|Default|GetSpringArm) (+ (Variables|/Script/Engine.SpringArmComponent|GetTargetArmLength (Variables|Default|GetSpringArm)) (select (== AxisValue 1.0) -5e+01 5e+01)))))

(fn ConstructionScript)

(fn CalculateEnergy
  (params (MinusEnergy :type Float%20%28single-precision%29))
  (if (>= (- (Variables|Default|GetEnergy) MinusEnergy) 0.0)
    (Variables|Default|SetEnergy (- (Variables|Default|GetEnergy) MinusEnergy))
    (return true)
    (else
      (return false))))