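; Base tower actor for a tower-defense game that targets Enemy_AI actors inside its capsule overlap and shoots them.
; Each tick the turret rotates toward the first listed target and, once aligned and past the fire interval, calls Fire, which waits RateFire before spawning a homing-target bullet.
; Construction loads level stats from DT_LvlTowerInfo, supplying bullet damage.
; The base highlights on hover and opens the WD_UpdateTower widget with UI-only input on click.
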(event OnComponentBeginOverlap(Capsule)
  (params (OverlappedComponent :type Primitive%20Component%20Object%20Reference) (OtherActor :type Actor%20Object%20Reference) (OtherComp :type Primitive%20Component%20Object%20Reference) (OtherBodyIndex :type Integer) (bFromSweep :type Boolean) (SweepResult :type Hit%20Result%20Structure%20%28by%20ref%29))
  (bind _asenemy_ai (Utilities|Casting|CastToEnemy_AI OtherActor))
  (Utilities|Array|Add (Variables|Default|GetTargetList) _asenemy_ai))

(event OnComponentEndOverlap(Capsule)
  (params (OverlappedComponent :type Primitive%20Component%20Object%20Reference) (OtherActor :type Actor%20Object%20Reference) (OtherComp :type Primitive%20Component%20Object%20Reference) (OtherBodyIndex :type Integer))
  (bind _asenemy_ai (Utilities|Casting|CastToEnemy_AI OtherActor))
  (Utilities|Array|RemoveItem (Variables|Default|GetTargetList) _asenemy_ai))

(event OnClicked(Tower_Osnova)
  (params (TouchedComponent :type Primitive%20Component%20Object%20Reference) (ButtonPressed :type Key%20Structure :default "None"))
  (bind _tower_osnova (Variables|Default|GetTower_Osnova))
  (if true
    (Rendering|Material|SetMaterial _tower_osnova 0 "/Game/TowerContent/Towers/Materials/Green.Green")
    (bind _returnvalue (UserInterface|CreateWidget "/Game/TowerContent/Towers/Widgets/WD_UpdateTower.WD_UpdateTower_C" 0 self))
    (UserInterface|Viewport|AddtoViewport _returnvalue 0)
    (Input|SetInputModeUIOnly (Game|GetPlayerController 0) 0 "DoNotLock")
    (else
      (Rendering|Material|SetMaterial _tower_osnova 0 "/Game/TowerContent/Towers/Materials/Red.Red"))))

(event OnReleased(Tower_Osnova)
  (params (TouchedComponent :type Primitive%20Component%20Object%20Reference) (ButtonReleased :type Key%20Structure :default "None")))

(event OnEndCursorOver(Tower_Osnova)
  (params (TouchedComponent :type Primitive%20Component%20Object%20Reference))
  (Rendering|Material|SetMaterial (Variables|Default|GetTower_Osnova) 0 "/Game/TowerContent/Towers/Materials/Black.Black"))

(event OnBeginCursorOver(Tower_Osnova)
  (params (TouchedComponent :type Primitive%20Component%20Object%20Reference))
  (Rendering|Material|SetMaterial (Variables|Default|GetTower_Osnova) 0 "/Game/TowerContent/Towers/Materials/Yellow.Yellow"))

(event Custom|Fire
  (Utilities|FlowControl|Delay (Variables|Default|GetRate%20Fire))
  (Variables|Default|SetTime%20Last%20Fire (Utilities|Time|GetGameTimeinSeconds))
  (Utilities|IsValid (Utilities|Array|Get(acopy) (Variables|Default|GetTargetList))
    (:Is%20Valid
      (bind _returnvalue (Game|SpawnActorfromClass "/Game/TowerContent/Towers/Bullet.Bullet_C" (Transformation|GetWorldTransform (Variables|Default|GetFirePoint)) "Undefined" 0 (.Damage (Utilities|Struct|BreakStruct_Info (Variables|Default|GetOut%20Row))) 0))
      (Variables|/Game/TowerContent/Towers/Bullet.Bullet_C|SetTarget _returnvalue (Utilities|Array|Get(acopy) (Variables|Default|GetTargetList))))))

(event EventTick
  (params (DeltaSeconds :type Float%20%28single-precision%29))
  (Utilities|IsValid (Utilities|Array|Get(acopy) (Variables|Default|GetTargetList))
    (:Is%20Valid
      (CallFunction|RotateTower DeltaSeconds)
      (CallFunction|FireEnemy))))

(event EventBeginPlay
  (bind _asbp_cam (Utilities|Casting|CastToBP_Cam (Game|Player|GetPlayerPawn 0)))
  (Variables|Default|SetBP%20Cam _asbp_cam))

(fn ConstructionScript
  (CallFunction|TakeInfoOutData))

(fn FireEnemy
  (if (> (- (Utilities|Time|GetGameTimeinSeconds) (Variables|Default|GetTime%20Last%20Fire)) (Variables|Default|GetRate%20Fire))
    (if (> (Math|Vector|DotProduct (Math|Vector|GetUnitDirection(Vector) (Transformation|GetWorldLocation (Variables|Default|GetTurrel)) (Transformation|GetActorLocation (Utilities|Array|Get(acopy) (Variables|Default|GetTargetList)))) (Math|Vector|GetForwardVector (Variables|Default|GetTurrel))) 0.99)
      (CallFunction|Fire))))

(fn RotateTower
  (params (NewParam :type Float%20%28single-precision%29))
  (Transformation|SetWorldRotation (Variables|Default|GetTurrel) (Class|KismetMathLibrary|RInterptoConstant (Transformation|GetWorldRotation (Variables|Default|GetTurrel)) (Math|Rotator|FindLookatRotation (Transformation|GetWorldLocation (Variables|Default|GetTurrel)) (Transformation|GetActorLocation (Utilities|Array|Get(acopy) (Variables|Default|GetTargetList)))) NewParam (Variables|Default|GetInterp%20Speed)) false false))

(fn TakeInfoOutData
  (bind _returnvalue (Utilities|GetDataTableRow "/Game/TowerContent/Towers/Tower/DT_LvlTowerInfo.DT_LvlTowerInfo" (Utilities|String|StringToName (Utilities|String|EnumtoString (Variables|Default|GetLevelTowerEnum))))
    (:then
      (Variables|Default|SetOut%20Row _returnvalue))))